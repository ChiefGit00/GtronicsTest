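; PickUp is a pickup actor whose type, Ammo, Health or Bullet Time, determines the static mesh it displays.
; The construction script applies the mesh for the current type, and the SetPickUpType event stores a new type and repeats the same switch.
; The file contains only this visual setup, with no overlap, collection or effect logic.
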(event `self.SetPickUpType`
  (params (PickUp :type "EPickUpType Enum" :default "Ammo"))
  (bind _mesh (`self.Mesh`))
  (bind _output_get (set `self.PickUpType` PickUp))
  (switch `EPickUpType` _output_get
    (:`Ammo`
      (`StaticMeshComponent.SetStaticMesh` _mesh "/Game/StaticMeshes/Bullets.Bullets"))
    (:`Health`
      (`StaticMeshComponent.SetStaticMesh` _mesh "/Game/StaticMeshes/Sphere/TwinStickProjectile.TwinStickProjectile"))
    (:`BulletTime`
      (`StaticMeshComponent.SetStaticMesh` _mesh "/Game/StaticMeshes/SpherePickUp.SpherePickUp"))))

(fn `UserConstructionScript`
  (bind _mesh (`self.Mesh`))
  (bind _output_get (set `self.PickUpType` (`self.PickUpType`)))
  (switch `EPickUpType` _output_get
    (:`Ammo`
      (`StaticMeshComponent.SetStaticMesh` _mesh "/Game/StaticMeshes/Bullets.Bullets"))
    (:`Health`
      (`StaticMeshComponent.SetStaticMesh` _mesh "/Game/StaticMeshes/Sphere/TwinStickProjectile.TwinStickProjectile"))
    (:`BulletTime`
      (`StaticMeshComponent.SetStaticMesh` _mesh "/Game/StaticMeshes/SpherePickUp.SpherePickUp"))))