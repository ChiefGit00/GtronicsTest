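; Game controller that manages the HUD and game-over screen and handles the restart key.
; It creates the game HUD widget and adds it to the viewport at BeginPlay.
; GameOver creates and shows the game-over widget unless one is already on screen, then passes it the kill count.
; Pressing R calls Restart on that widget if it exists, and an unconnected branch holds unused HUD removal.
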(event `self.ReceiveBeginPlay`
  (bind _returnvalue (`|CreateWidget` "/Game/UI/WB_GameHUD.WB_GameHUD_C"))
  (bind _output_get (set `self.HUD` _returnvalue))
  (`UserWidget.AddToViewport` _output_get 0))

(event `self.GameOver`
  (params (Kills :type Integer))
  (bind _gameoverui (`self.GameOverUI`))
  (`/Engine/EditorBlueprintResources/StandardMacros.IsValid` _gameoverui
    (:`Is Valid`
      (if (not (`Widget.IsInViewport` _gameoverui))
        (bind _returnvalue (`|CreateWidget` "/Game/UI/WB_GameOVer.WB_GameOver_C" :!label _label))
        (bind _output_get (set `self.GameOverUI` _returnvalue))
        (`UserWidget.AddToViewport` _output_get 0)
        (`/Game/UI/WB_GameOVer.Kills` _returnvalue Kills)))
    (:`Is Not Valid`
      (goto _label))))

(event `Key|R`
  (params (Key :type "Key Structure"))
  (bind _gameoverui (`self.GameOverUI`))
  (:`Pressed`
    (`/Engine/EditorBlueprintResources/StandardMacros.IsValid` _gameoverui
      (:`Is Valid`
        (`W_GameOver.Restart` _gameoverui)))))

(fn `UserConstructionScript`)